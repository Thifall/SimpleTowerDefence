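; Tower defence enemy that walks an ordered list of path nodes and destroys itself after the last one.
; Each tick moves the Cylinder component without sweep along the vector from the segment's saved start to the current node.
; That vector is not normalised, so speed scales with segment length.
; A tight 2D distance check advances the node index and re-saves the actor transform as the next start.
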(event `self.ReceiveBeginPlay`
  (set `self.StartingLocation` (`self.GetTransform`)))

(event `self.ReceiveTick`
  (params (DeltaSeconds :type "Float (single-precision)"))
  (bind _startinglocation_location (`KismetMathLibrary.BreakTransform` (`self.StartingLocation`)))
  (bind _returnvalue_location (`KismetMathLibrary.BreakTransform` (`SceneComponent.K2_GetComponentToWorld` (`self.Cylinder`))))
  (bind _output (`|GetArrayItem` (`self.PathNodes`) (`self.CurrentPathNodeIndex`)))
  (bind _returnvalue_location_2 (`KismetMathLibrary.BreakTransform` (`self.GetTransform` _output)))
  (bind _returnvalue_location_3 (`KismetMathLibrary.BreakTransform` (`self.GetTransform` _output)))
  (if (< (`self.CurrentPathNodeIndex`) (`KismetArrayLibrary.Array_Length` (`self.PathNodes`)))
    (if (< (`KismetMathLibrary.Distance2D` (`KismetMathLibrary.Conv_VectorToVector2D` _returnvalue_location) (`KismetMathLibrary.Conv_VectorToVector2D` _returnvalue_location_3)) 1.0)
      (`KismetSystemLibrary.PrintText` "Stopping!")
      (set `self.CurrentPathNodeIndex` (+ (`self.CurrentPathNodeIndex`) 1))
      (set `self.StartingLocation` (`self.GetTransform`))
      (else
        (`SceneComponent.K2_AddRelativeLocation` (`self.Cylinder`) (* (* (- _returnvalue_location_2 _startinglocation_location) DeltaSeconds) (`self.MoveSpeed`)) false false)))
    (else
      (`self.K2_DestroyActor`))))

(fn `UserConstructionScript`)